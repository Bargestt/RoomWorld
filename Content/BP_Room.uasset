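; BP_Room is a room node that links to other nodes through sockets and can load itself at game start.
; With AutoLoad on, it waits briefly for the RoomManager to initialise, then sets its state to Visible.
; When its level is shown, it walks each socket's connections and snaps every valid, movable connected node onto the matching socket of this room.
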(event `self.ReceiveBeginPlay`
  (if (`self.bAutoLoad`)
    (`KismetSystemLibrary.Delay` 0.2) ; Wait initalisation in RoomManager
    (`self.SetState` "Visible")))

(event `self.ReceiveLevelShown`
  (`self.SnapConnected`))

(event `SnapConnected`
  (for _array_element (`self.GetRoomSockets`)
    (for _array_element_2 (`RoomSocket.GetConnections` _array_element)
      (`/Engine/EditorBlueprintResources/StandardMacros.IsValid` _array_element_2
        (:`Is Valid`
          (bind _returnvalue (`RoomSocket.GetNode` _array_element_2))
          (`/Engine/EditorBlueprintResources/StandardMacros.IsValid` _returnvalue
            (:`Is Valid`
              (if (`self.CanMove` _returnvalue)
                (`self.SnapWithNode` _returnvalue (`RoomSocket.Name` _array_element_2) self (`RoomSocket.Name` _array_element))))))))))

(fn `UserConstructionScript`)