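; BP_RoomWorldTestPlayer is a test player character with an orbit-style spring-arm camera and direct keyboard controls.
; Mouse axes drive controller yaw and pitch, while the wheel sets a clamped zoom distance that Tick smoothly interpolates onto the spring arm.
; WASD and Space toggle Gates in a Tick sequence, feeding camera-relative horizontal movement input and a continuous upward force on CharacterMovement while held.
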(event `InputAxisKey|MouseWheelAxis`
  (params (AxisValue :type "Float (single-precision)"))
  (set `self.CameraDist` (`KismetMathLibrary.FClamp` (+ (* AxisValue -100.0) (`self.CameraDist`)) 500.0 3000.0)))

(event `InputAxisKey|MouseX`
  (params (AxisValue :type "Float (single-precision)"))
  (`self.AddControllerYawInput` (* AxisValue 1.0)))

(event `InputAxisKey|MouseY`
  (params (AxisValue :type "Float (single-precision)"))
  (`self.AddControllerPitchInput` (* AxisValue -1.0)))

(event `self.ReceiveTick`
  (params (DeltaSeconds :type "Float (single-precision)"))
  (bind _springarm (`self.SpringArm`))
  (bind _returnvalue (* (`KismetMathLibrary.Vector_Normal2D` (`SceneComponent.GetForwardVector` (`self.Camera`))) 100.0))
  (bind _returnvalue_2 (* (`KismetMathLibrary.Vector_Normal2D` (`SceneComponent.GetRightVector` (`self.Camera`))) 100.0))
  (`|ExecutionSequence`
    (:`then_0`
      (set `SpringArmComponent.TargetArmLength` (`KismetMathLibrary.FInterpTo` (`SpringArmComponent.TargetArmLength` _springarm) (`self.CameraDist`) (`GameplayStatics.GetWorldDeltaSeconds`) 10.0) _springarm))
    (:`then_1`
      (`/Engine/EditorBlueprintResources/StandardMacros.Gate` true :!label _label
        (:`Exit`
          (`self.AddMovementInput` _returnvalue (`GameplayStatics.GetWorldDeltaSeconds`)))))
    (:`then_2`
      (`/Engine/EditorBlueprintResources/StandardMacros.Gate` true :!label _label_2
        (:`Exit`
          (`self.AddMovementInput` (`KismetMathLibrary.NegateVector` _returnvalue) (`GameplayStatics.GetWorldDeltaSeconds`)))))
    (:`then_3`
      (`/Engine/EditorBlueprintResources/StandardMacros.Gate` true :!label _label_3
        (:`Exit`
          (`self.AddMovementInput` _returnvalue_2 (`GameplayStatics.GetWorldDeltaSeconds`)))))
    (:`then_4`
      (`/Engine/EditorBlueprintResources/StandardMacros.Gate` true :!label _label_4
        (:`Exit`
          (`self.AddMovementInput` (`KismetMathLibrary.NegateVector` _returnvalue_2) (`GameplayStatics.GetWorldDeltaSeconds`)))))
    (:`then_5`
      (`/Engine/EditorBlueprintResources/StandardMacros.Gate` true :!label _label_5
        (:`Exit`
          (`CharacterMovementComponent.AddForce` (`self.CharacterMovement`) (0.0 0.0 200000.0)))))))

(event `Key|W`
  (params (Key :type "Key Structure"))
  (:`Pressed`
    (goto _label :!via `Open`))
  (:`Released`
    (goto _label :!via `Close`)))

(event `Key|S`
  (params (Key :type "Key Structure"))
  (:`Pressed`
    (goto _label_2 :!via `Open`))
  (:`Released`
    (goto _label_2 :!via `Close`)))

(event `Key|D`
  (params (Key :type "Key Structure"))
  (:`Pressed`
    (goto _label_3 :!via `Open`))
  (:`Released`
    (goto _label_3 :!via `Close`)))

(event `Key|A`
  (params (Key :type "Key Structure"))
  (:`Pressed`
    (goto _label_4 :!via `Open`))
  (:`Released`
    (goto _label_4 :!via `Close`)))

(event `Key|SpaceBar`
  (params (Key :type "Key Structure"))
  (:`Pressed`
    (goto _label_5 :!via `Open`))
  (:`Released`
    (goto _label_5 :!via `Close`)))

(fn `UserConstructionScript`)