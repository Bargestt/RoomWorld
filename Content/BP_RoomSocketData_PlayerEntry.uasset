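; BP_RoomSocketData_PlayerEntry is room socket data that tracks players crossing a room entry point.
; When given its owning room, it caches that room's RoomPlayerInfo component.
; RoomEntryPoint crossing events are forwarded to that component as player entered or left, provided it is valid.
; The construction script sizes the Box from Extent, enforcing a minimum X width.
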(event `self.RoomEntryPoint.OnPlayerHasCrossed`
  (params (Point :type "/RoomWorld/Components/RoomEntryPoint Object Reference") (Player :type "PlayerController Object Reference") (bHasEntered :type Boolean))
  (bind _playerinfo (`self.PlayerInfo`)
    (:`then`
      (if bHasEntered
        (`/RoomWorld/Components/RoomPlayerInfo.PlayerEntered` _playerinfo Player)
        (else
          (`/RoomWorld/Components/RoomPlayerInfo.PlayerLeft` _playerinfo Player))))
    (:`else`)))

(event `RoomOwnedObjectInterface.SetOwningRoom`
  (params (Room :type "Room Object Reference"))
  (set `self.PlayerInfo` (`self.GetComponentByClass` Room "/RoomWorld/Components/RoomPlayerInfo.RoomPlayerInfo_C")))

(fn `UserConstructionScript`
  (bind _output_get (set `self.Extent` (`KismetMathLibrary.MakeVector` (`KismetMathLibrary.FMax` (`self.MinWidth`) (.x (`self.Extent`))) (.y (`self.Extent`)) (.z (`self.Extent`)))))
  (`BoxComponent.SetBoxExtent` (`self.Box`) _output_get true))