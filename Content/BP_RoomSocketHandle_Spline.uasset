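; Room socket handle that shows its connection as a colored spline mesh, hidden in game while its room is Visible and shown when Loaded or Unloaded.
; Connection and node events, plus construction, refresh color via custom primitive data and reshape the spline.
; The spline fits a full curve to the connected handle, then trims it to the midpoint, leaving a short stub if unconnected.
; Construction also reshapes the connected handle's spline.
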(event `self.ReceiveBeginPlay`
  (bind _asroom (cast `Room` (`RoomSocketHandleFunctionLibrary.GetNode`)))
  (add `Room.OnStateChanged` _asroom (delegate `OnStateChanged`)))

(event `OnStateChanged`
  (params (Room :type "Room Object Reference") (NewState :type "ERoomState Enum" :default "Unloaded"))
  (switch `ERoomState` NewState
    (:`Unloaded`
      (`self.SetActorHiddenInGame` false :!label _label))
    (:`Loaded`
      (goto _label))
    (:`Visible`
      (`self.SetActorHiddenInGame` true))))

(event `self.ReceiveConnectionGained`
  (params (NewConnection :type "RoomSocket Object Reference") (Index :type Integer))
  (`self.Check` :!label _label_2)
  (`self.UpdateSplineShape`))

(event `self.ReceiveConnectionLost`
  (params (OldConnection :type "RoomSocket Object Reference") (Index :type Integer))
  (goto _label_2))

(event `self.ReceiveConnectionMoved`
  (params (Index :type Integer))
  (goto _label_2))

(event `self.ReceiveNodeMoved`
  (goto _label_2))

(fn `Check`
  (locals (UseColor :type "LinearColor Structure") (Connections :type "Array of RoomSocket Object Reference"))
  (bind _output_get (set `local.Connections` (`RoomSocketHandleFunctionLibrary.GetConnections`)))
  (`KismetArrayLibrary.Array_RemoveItem` _output_get)
  (bind _output_get_2 (set `local.UseColor` (`KismetMathLibrary.SelectColor` (`self.Color_Connected`) (`self.Color_Free`) (> (`KismetArrayLibrary.Array_Length` _output_get) 0))))
  (`self.SetColor` _output_get_2))

(fn `SetColor`
  (params (LinearColor :type "LinearColor Structure (by ref)"))
  (locals (V4 :type "Vector4 Structure"))
  (bind (_r _g _b _a) (break `LinearColor` LinearColor))
  (bind _base (`self.Base`))
  (bind _spline (`self.Spline`))
  (bind _output_get (set `local.V4` (`KismetMathLibrary.MakeVector4` _r _g _b _a)))
  (`|ExecutionSequence`
    (:`then_0`
      (`PrimitiveComponent.SetDefaultCustomPrimitiveDataVector4` _base 0 _output_get)
      (`PrimitiveComponent.SetCustomPrimitiveDataVector4` _base 0 _output_get))
    (:`then_1`
      (`PrimitiveComponent.SetDefaultCustomPrimitiveDataVector4` _spline 0 _output_get)
      (`PrimitiveComponent.SetCustomPrimitiveDataVector4` _spline 0 _output_get))))

(fn `UpdateSplineShape`
  (locals (End :type "Vector Structure" :default (0.0 0.0 0.0)))
  (bind _spline (`self.Spline`))
  (bind _returnvalue (`SceneComponent.K2_GetComponentToWorld` (`self.Spline`)))
  (bind _returnvalue_2 (`RoomSocketHandleFunctionLibrary.GetSocketHandle` (`RoomSocketHandleFunctionLibrary.GetConnection` 0)))
  (`/Engine/EditorBlueprintResources/StandardMacros.IsValid` _returnvalue_2
    (:`Is Valid`
      (bind _output_get (set `local.End` (`KismetMathLibrary.InverseTransformLocation` _returnvalue (`self.K2_GetActorLocation` _returnvalue_2))))
      (bind _returnvalue_3 (* (`KismetMathLibrary.VSize` _output_get) 2.0))
      (`SplineMeshComponent.SetStartAndEnd` _spline (0.0 0.0 0.0) (* (1.0 0.0 0.0) _returnvalue_3) _output_get (* (`KismetMathLibrary.InverseTransformDirection` _returnvalue (`KismetMathLibrary.NegateVector` (`self.GetActorForwardVector` _returnvalue_2))) _returnvalue_3) false)
      (bind _returnvalue_4 (`RoomWorldFunctionLibrary.CalcSliceTransformAtSplineOffset` _spline 0.5))
      (`SplineMeshComponent.SetStartAndEnd` _spline (0.0 0.0 0.0) (* (`SplineMeshComponent.GetStartTangent` _spline) 0.5) (.location _returnvalue_4) (0.0 0.0 0.0) true))
    (:`Is Not Valid`
      (set `local.End` (100.0 0.0 0.0))
      (`SplineMeshComponent.SetStartAndEnd` (`self.Spline`) (0.0 0.0 0.0) (0.0 0.0 0.0) (0.0 0.0 0.0) (0.0 0.0 0.0) true))))

(fn `UserConstructionScript`
  (`self.Check`)
  (`self.UpdateSplineShape`)
  (bind _asroom_socket_spline (cast `/Game/BP_RoomSocketHandle_Spline` (`RoomSocketHandleFunctionLibrary.GetSocketHandle` (`RoomSocketHandleFunctionLibrary.GetConnection` 0))))
  (`self.UpdateSplineShape` _asroom_socket_spline))