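; Room manager that controls which Room nodes are visible around players and persists the current room in a save slot.
; On BeginPlay it loads the save, which can override InitialRoom, then optionally moves that room to a configurable origin and makes it visible.
; Player enter and leave events diff occupied rooms plus connected neighbors against VisibleRooms to request or clear visibility.
; Entering records the current room and can auto-save.
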(event `LoadInitialRoom`
  (bind (_location _rotation) (`self.GetOrigin`))
  (bind _initialroom (`self.InitialRoom`)
    (:`then`
      (`|ExecutionSequence`
        (:`then_0`
          (if (`self.bMoveInitialRoom`)
            (`self.K2_SetActorLocationAndRotation` _initialroom _location _rotation false false)))
        (:`then_1`
          (`Room.SetState` _initialroom "Visible"))))
    (:`else`)))

(event `OnStateChanged_Room`
  (params (Room :type "Room Object Reference") (NewState :type "ERoomState Enum" :default "Unloaded"))
  (bind _initialroom (`self.InitialRoom`)
    (:`then`
      (if (and (== Room _initialroom) (`|EnumEquality` NewState "Visible"))
        (`self.OnInitialRoomLoaded`)))
    (:`else`)))

(event `self.ReceiveBeginPlay`
  (`|ExecutionSequence`
    (:`then_0`
      (`self.LoadState`))
    (:`then_1`
      (bind _outnodes (`self.GetAllNodesOfClass` "/Script/RoomWorld.Room"))
      (for _array_element _outnodes
        (add `Room.OnStateChanged` _array_element (`|CreateDelegate` :!event `OnStateChanged_Room`))))
    (:`then_2`
      (`self.LoadInitialRoom`))))

(event `self.RoomPlayerInfo.PlayerEnter`
  (params (Info :type "/RoomWorld/Components/RoomPlayerInfo Object Reference"))
  (`|ExecutionSequence`
    (:`then_0`
      (bind _output_get (set `/RoomWorld/BP_RoomWorldSaveGame.CurrentRoom` (`|ConvertAsset` (`/RoomWorld/Components/RoomPlayerInfo.GetRoom` Info)) (`self.State`)))
      (`self.Msg` (`KismetStringLibrary.Concat_StrStr` "CurrentRoom: " (`BlueprintPathsLibrary.GetExtension` (`KismetSystemLibrary.Conv_SoftObjectReferenceToString` _output_get))))
      (if (`self.bAutoSaveOnEnter`)
        (`self.SaveState`)))
    (:`then_1`
      (`self.UpdateRoomsVisibleToPlayers` :!label _label))))

(event `self.RoomPlayerInfo.PlayerLeave`
  (params (Info :type "/RoomWorld/Components/RoomPlayerInfo Object Reference"))
  (goto _label))

(fn `GetOrigin`
  (returns (Location :type "Vector Structure") (Rotation :type "Rotator Structure"))
  (bind _originoffsetrot (`self.OriginOffsetRot`))
  (bind _originoffsetloc (`self.OriginOffsetLoc`))
  (bind _originactor (`self.OriginActor`)
    (:`then`
      (return (.location (`KismetMathLibrary.ComposeTransforms` (`KismetMathLibrary.MakeTransform` _originoffsetloc _originoffsetrot) (`self.GetTransform` _originactor))) (.rotation (`KismetMathLibrary.ComposeTransforms` (`KismetMathLibrary.MakeTransform` _originoffsetloc _originoffsetrot) (`self.GetTransform` _originactor)))))
    (:`else`
      (return _originoffsetloc _originoffsetrot))))

(fn `GetSaveSlotName`
  (returns (bCanSave :type Boolean) (SlotName :type String))
  (bind _slotname (`self.SlotName`))
  (return (not (`KismetStringLibrary.IsEmpty` _slotname)) _slotname))

(fn `InitSave`)

(fn `LoadState`
  (locals (Name :type String))
  (bind (_bcansave _slotname) (`self.GetSaveSlotName`))
  (if _bcansave
    (bind _returnvalue (`GameplayStatics.LoadGameFromSlot` _slotname))
    (bind _asbp_room_world_save_game (cast `/RoomWorld/BP_RoomWorldSaveGame` _returnvalue)
      (:`then`
        (set `self.State` _asbp_room_world_save_game)
        (`self.PostLoad`))
      (:`CastFailed`
        (bind _returnvalue_2 (`GameplayStatics.CreateSaveGameObject` (`self.StateClass`) :!label _label))
        (set `self.State` _returnvalue_2)
        (`self.InitSave`)))
    (else
      (goto _label))))

(fn `Msg`
  (params (Msg :type String) (bError :type Boolean))
  (`KismetSystemLibrary.PrintString` (`KismetStringLibrary.Concat_StrStr` "[" (`KismetSystemLibrary.GetDisplayName` self) "]  " Msg) (`self.bDebug`) false (`KismetMathLibrary.SelectColor` (struct :`R` 1.0 :`A` 1.0) (struct :`G` 1.0 :`B` 0.817953 :`A` 1.0) bError) 5.0))

(fn `PostLoad`
  (bind _output (`|ConvertAsset` (`/RoomWorld/BP_RoomWorldSaveGame.CurrentRoom` (`self.State`))))
  (if (`KismetSystemLibrary.IsValid` _output)
    (bind _output_get (set `self.InitialRoom` _output))
    (`self.Msg` (`KismetStringLibrary.Concat_StrStr` "Loaded to room: " (`KismetSystemLibrary.GetDisplayName` _output_get)))))

(fn `ResetState`
  (bind (_bcansave _slotname) (`self.GetSaveSlotName`))
  (if _bcansave
    (`GameplayStatics.DeleteGameInSlot` _slotname))
  (bind _returnvalue (`GameplayStatics.CreateSaveGameObject` (`self.StateClass`)))
  (set `self.State` _returnvalue)
  (`self.InitSave`)
  (`self.Msg` "Reset"))

(fn `SaveState`
  (locals (Name :type String))
  (bind (_bcansave _slotname) (`self.GetSaveSlotName`))
  (if _bcansave
    (bind _returnvalue (`GameplayStatics.SaveGameToSlot` (`self.State`) _slotname))
    (if _returnvalue
      (`self.Msg` "Save success")
      (else
        (`self.Msg` "Save failed" true)))))

(fn `UpdateRoomsVisibleToPlayers`
  (locals (RelevantRooms :type "Set of Room Object Reference"))
  (bind _relevantrooms (`local.RelevantRooms`))
  (bind _playerrooms (`/RoomWorld/Components/RoomPlayerInfo.GetPlayerRooms` (`self.RoomPlayerInfo`)))
  (for _array_element _playerrooms
    (`BlueprintSetLibrary.Set_Add` _relevantrooms _array_element)
    (bind _nodes (`RoomNode.BP_GetConnectedNodes` _array_element "/Script/RoomWorld.Room"))
    (`BlueprintSetLibrary.Set_AddItems` _relevantrooms _nodes))
  (if (> (`KismetArrayLibrary.Array_Length` _playerrooms) 0)
    (bind _result (`BlueprintSetLibrary.Set_Difference` (`self.VisibleRooms`) (`local.RelevantRooms`)))
    (bind _result_2 (`BlueprintSetLibrary.Set_ToArray` _result))
    (`BlueprintSetLibrary.Set_RemoveItems` (`self.VisibleRooms`) _result_2)
    (`Room.ClearVisible` _result_2 self)
    (bind _result_3 (`BlueprintSetLibrary.Set_ToArray` (`local.RelevantRooms`)))
    (`BlueprintSetLibrary.Set_AddItems` (`self.VisibleRooms`) _result_3)
    (`Room.RequestVisible` _result_3 self)))

(fn `UserConstructionScript`)